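; Openable door actor Blueprint that swings open and closed in response to the OpenDoor component's OnOpen and OnClose events.
; On BeginPlay it stores its starting rotation, and the DoorSwing timeline adds its SwingAngle yaw to that rotation on each update.
; Opening plays the timeline, whose Play Sound event track triggers a lock sound at the door, and closing reverses it.
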(event OnClose(OpenDoor)
  (bind _swingangle (Timeline|Door%20Swing Reverse)
    (:Update
      (Transformation|SetActorRotation (Math|Rotator|CombineRotators (Math|Rotator|MakeRotator 0.0 0.0 _swingangle) (Variables|Default|GetInitial%20Rotation))))
    (:Play%20Sound
      (Audio|PlaySoundatLocation "/Game/Audio/door-lock.door-lock" (Transformation|GetActorLocation)))))

(event OnOpen(OpenDoor)
  (bind _swingangle (Timeline|Door%20Swing Play)
    (:Update
      (Transformation|SetActorRotation (Math|Rotator|CombineRotators (Math|Rotator|MakeRotator 0.0 0.0 _swingangle) (Variables|Default|GetInitial%20Rotation))))
    (:Play%20Sound
      (Audio|PlaySoundatLocation "/Game/Audio/door-lock.door-lock" (Transformation|GetActorLocation)))))

(event EventBeginPlay
  (Variables|Default|SetInitial%20Rotation (Transformation|GetActorRotation)))

(fn ConstructionScript)

(fn SetBlueprintVariables
  (params (DoorLocation :type Vector) (Initial%20Rotation :type Rotator)))